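; Player character Blueprint with look and move helpers, a weapon that attaches to equip or unequip sockets, and melee combo attacks.
; BeginPlay spawns BP_Weapon on the UnEquip socket, and separate functions move it between sockets or set the current pose state.
; Attack cycles three AM_Attack montage sections through a counter.
; BattleForm's branch is hardwired true, so it always applies battle speed, and Tick prints max walk speed for debugging.
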(event EventBeginPlay
  (bind _returnvalue (Game|SpawnActorfromClass "/Game/BP/Player/Weapon/BP_Weapon.BP_Weapon_C" (Math|Transform|MakeTransform "0, 0, 0") "AdjustIfPossibleButAlwaysSpawn" "MultiplyWithRoot" 0 0))
  (Variables|Default|SetWeaponRef _returnvalue)
  (Transformation|AttachComponentToComponent (Variables|Default|GetWeaponRef) (Variables|Character|GetMesh) "UnEquip" "SnapToTarget" "SnapToTarget" "KeepWorld" false))

(event Collision|EventActorBeginOverlap
  (params (OtherActor :type Actor%20Object%20Reference)))

(event EventTick
  (params (DeltaSeconds :type Float%20%28single-precision%29))
  (Development|PrintString (Utilities|String|ToString(Text) (Utilities|Text|FormatText "Movement : {0}" (Variables|/Script/Engine.CharacterMovementComponent|GetMaxWalkSpeed (Variables|Character|GetCharacterMovement)))) true true "(R=0.000000,G=0.660000,B=1.000000,A=1.000000)" 0.0))

(fn ConstructionScript)

(fn InputLook
  (params (bIsTurn :type Boolean) (Axis%20Value :type Float%20%28double-precision%29))
  (if bIsTurn
    (Pawn|Input|AddControllerYawInput Axis%20Value)
    (else
      (Pawn|Input|AddControllerPitchInput Axis%20Value))))

(fn InputMove
  (params (bIsForward :type Boolean) (AxisValue :type Float%20%28double-precision%29))
  (bind _returnvalue (Pawn|GetController))
  (if bIsForward
    (Pawn|Input|AddMovementInput (Transformation|GetActorForwardVector _returnvalue) AxisValue false)
    (else
      (Pawn|Input|AddMovementInput (Transformation|GetActorRightVector _returnvalue) AxisValue false))))

(fn BattleForm
  (bind _charactermovement (Variables|Character|GetCharacterMovement))
  (bind _charactermovement_2 (Variables|Character|GetCharacterMovement))
  (if true
    (bind _output_get (Variables|/Script/Engine.CharacterMovementComponent|SetMaxWalkSpeed _charactermovement_2 (Variables|Default|GetWeaponBattleSpeed)))
    (Variables|/Script/Engine.CharacterMovementComponent|SetMaxAcceleration _charactermovement_2 _output_get)
    (else
      (bind _output_get_2 (Variables|/Script/Engine.CharacterMovementComponent|SetMaxWalkSpeed _charactermovement (Variables|Default|GetUnarmedWalkSpeed)))
      (Variables|/Script/Engine.CharacterMovementComponent|SetMaxAcceleration _charactermovement _output_get_2))))

(fn Attack
  (switch int (Variables|Attack|GetComboAttackCounter)
    (:0
      (Animation|PlayAnimMontage "/Game/BP/Player/Anim/AM/AM_Attack.AM_Attack" 1.0 "Combo1")
      (Variables|Attack|SetComboAttackCounter (+ 1 (Variables|Attack|GetComboAttackCounter))))
    (:1
      (Animation|PlayAnimMontage "/Game/BP/Player/Anim/AM/AM_Attack.AM_Attack" 1.0 "Combo2")
      (Variables|Attack|SetComboAttackCounter (+ 1 (Variables|Attack|GetComboAttackCounter))))
    (:2
      (Animation|PlayAnimMontage "/Game/BP/Player/Anim/AM/AM_Attack.AM_Attack" 1.0 "Combo3")
      (Variables|Attack|SetComboAttackCounter 0))))

(fn UpdatePoseState
  (params (State :type E_PlayerState%20Enum :default "NewEnumerator0"))
  (Variables|Default|SetCurrentState State))

(fn EquipWeapon
  (Transformation|AttachComponentToComponent (Variables|Default|GetWeaponRef) (Variables|Character|GetMesh) "Equip" "SnapToTarget" "SnapToTarget" "KeepWorld" true))

(fn UnEquipWeapon
  (Transformation|AttachComponentToComponent (Variables|Default|GetWeaponRef) (Variables|Character|GetMesh) "UnEquip" "SnapToTarget" "SnapToTarget" "KeepWorld" true))